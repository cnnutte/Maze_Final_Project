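; Enemy AI pawn that chases the first-person player character on sight and plays audio during the pursuit.
; PawnSensing sightings issue an AI MoveTo and set a CanSeeEnemy flag, which a retriggerable delay clears shortly after sightings stop.
; A DoOnce starts the audio component created at BeginPlay.
; Tick rechecks the flag after a short delay, then fades the audio out and resets the DoOnce.
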(event OnSeePawn(PawnSensing)
  (params (Pawn :type Pawn%20Object%20Reference))
  (bind _asfirst_person_character (Utilities|Casting|CastToFirstPersonCharacter Pawn))
  (Utilities|FlowControl|Sequence
    (:then_0
      (Variables|Default|SetCan%20See%20Enemy? true)
      (AI|AIMoveTo self "0, 0, 0" _asfirst_person_character 5.0 false
        (:then
          (Utilities|FlowControl|DoOnce false
            (:Completed
              (Audio|Components|Audio|Play (Variables|Default|GetAudio) 0.0))))))
    (:then_1
      (Utilities|FlowControl|RetriggerableDelay 0.6)
      (Variables|Default|SetCan%20See%20Enemy? false))))

(event EventBeginPlay
  ;[1 1 1] Create Audio Reference
  (bind _returnvalue (AddComponent|AddAudioComponent false))
  (Audio|Components|Audio|Stop _returnvalue)
  (Variables|Default|SetAudio _returnvalue))

(event EventTick
  (params (DeltaSeconds :type Float%20%28single-precision%29))
  (if (not (Variables|Default|GetCan%20See%20Enemy?))
    (Utilities|FlowControl|Delay 0.4)
    (if (not (Variables|Default|GetCan%20See%20Enemy?))
      (Audio|Components|Audio|FadeOut (Variables|Default|GetAudio) 5.0 0.0 "Linear" :!class /Script/Engine.AudioComponent)
      (Utilities|FlowControl|DoOnce false) ; enters at Reset
    )))

(fn ConstructionScript)